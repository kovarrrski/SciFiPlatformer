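; Bat enemy that patrols endlessly back and forth between two marker components, TopPos and BottomPos.
; BeginPlay caches both markers' world locations, so the endpoints stay fixed while the actor moves, then sets the timeline play rate.
; The MoveAnim timeline lerps the actor's location without sweep, and a FlipFlop on Finished alternates reverse and forward playback instead of using Tick.
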(event Custom|MoveForward
  (bind _alpha (Timeline|MoveAnim PlayFromStart)
    (:Update
      (Transformation|SetActorLocation (Math|Vector|Lerp(Vector) (Variables|Default|GetWorldTopPos) (Variables|Default|GetWorldBottomPos) _alpha) false false))
    (:Finished
      ;[1 1 1] Cycles Timeline
      (Utilities|FlowControl|FlipFlop
        (:A
          (CallFunction|MoveBackward))
        (:B
          (CallFunction|MoveForward))))))

(event Custom|MoveBackward
  (bind _alpha (Timeline|MoveAnim ReverseFromEnd)
    (:Update
      (Transformation|SetActorLocation (Math|Vector|Lerp(Vector) (Variables|Default|GetWorldTopPos) (Variables|Default|GetWorldBottomPos) _alpha) false false))
    (:Finished
      ;[1 1 1] Cycles Timeline
      (Utilities|FlowControl|FlipFlop
        (:A
          (CallFunction|MoveBackward))
        (:B
          (CallFunction|MoveForward))))))

(event EventBeginPlay
  (|CallParentFunction)
  ;[1 1 1] Set Positions to vars for preventing of bugs
  (Variables|Default|SetWorldTopPos (Transformation|GetWorldLocation (Variables|Default|GetTopPos)))
  (Variables|Default|SetWorldBottomPos (Transformation|GetWorldLocation (Variables|Default|GetBottomPos)))
  ;[1 1 1] Speed of Movement x0.66
  (Components|Timeline|SetPlayRate (Variables|Default|GetMoveAnim) (Variables|Default|GetMovePlayRate))
  (CallFunction|MoveForward))

(event Collision|EventActorBeginOverlap
  (params (OtherActor :type Actor%20Object%20Reference))
  (|CallParentFunction OtherActor) ; This node is disabled and will not be called.\nDrag off pins to build functionality.
)

(event EventTick
  (params (DeltaSeconds :type Float%20%28single-precision%29))
  (|CallParentFunction DeltaSeconds) ; This node is disabled and will not be called.\nDrag off pins to build functionality.
)

(fn ConstructionScript
  (|CallParentFunction))