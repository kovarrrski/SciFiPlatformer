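; Lizard enemy character Blueprint that adds a fireball ranged attack.
; ShootFireball spawns a BP_EnemyProjectile_Lizard at the actor's center with the actor's rotation, always spawning regardless of collision.
; The event graph holds only disabled placeholder events and the construction script just calls the parent, so nothing in this file triggers the shot.
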(event EventBeginPlay
  (|CallParentFunction) ; This node is disabled and will not be called.\nDrag off pins to build functionality.
)

(event Collision|EventActorBeginOverlap
  (params (OtherActor :type Actor%20Object%20Reference))
  (|CallParentFunction OtherActor) ; This node is disabled and will not be called.\nDrag off pins to build functionality.
)

(event EventTick
  (params (DeltaSeconds :type Float%20%28single-precision%29))
  (|CallParentFunction DeltaSeconds) ; This node is disabled and will not be called.\nDrag off pins to build functionality.
)

(fn ConstructionScript
  (|CallParentFunction))

(fn ShootFireball
  (Game|SpawnActorfromClass "/Game/Blueprints/Projectiles/Enemy/BP_EnemyProjectile_Lizard.BP_EnemyProjectile_Lizard_C" (Math|Transform|MakeTransform (Transformation|GetActorLocation) (Transformation|GetActorRotation) "1.000000,1.000000,1.000000") "AlwaysSpawn" "MultiplyWithRoot" 0 0))