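; Checkpoint prop that registers itself as the active checkpoint in GM_SciFi when the player reaches it.
; BeginPlay caches the game mode, and the Trigger component's begin overlap filters for BP_Player.
; A DoOnce with no reset lets each checkpoint activate only once, writing itself to ActiveCheckpoint and switching the Cube to a green material.
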(event OnComponentBeginOverlap(Trigger)
  (params (OverlappedComponent :type Primitive%20Component%20Object%20Reference) (OtherActor :type Actor%20Object%20Reference) (OtherComp :type Primitive%20Component%20Object%20Reference) (OtherBodyIndex :type Integer) (bFromSweep :type Boolean) (SweepResult :type Hit%20Result%20Structure%20%28by%20ref%29))
  ;[1 1 1] Rewrite Active Checkpointin GM, Once when Player Overlap box
  (Utilities|Casting|CastToBP_Player OtherActor)
  (Utilities|FlowControl|DoOnce false
    (:Completed
      (Variables|/Game/Blueprints/GM_SciFi.GM_SciFi_C|SetActiveCheckpoint (Variables|Default|GetGM_SciFi) self)
      (Rendering|Material|SetMaterial (Variables|Default|GetCube) 0 "/AnimationSharing/AnimSharingGreen.AnimSharingGreen"))))

(event EventBeginPlay
  ;[1 1 1] Connection with GameMode
  (bind _asgm_sci_fi (Utilities|Casting|CastToGM_SciFi (Game|GetGameMode)))
  (Variables|Default|SetGM_SciFi _asgm_sci_fi))

(event Collision|EventActorBeginOverlap
  (params (OtherActor :type Actor%20Object%20Reference)))

(event EventTick
  (params (DeltaSeconds :type Float%20%28single-precision%29)))

(fn ConstructionScript)