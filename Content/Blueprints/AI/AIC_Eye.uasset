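; AI controller for the BP_Enemy_Eye enemy that tracks the direction from the eye to the player.
; On possess it caches the eye pawn, then after a short delay stores player pawn 0 as the target and prints its name.
; Each tick it computes the look-at forward vector toward that target and only prints it.
; A MoveTowards call along that vector is present but disconnected, so this controller does not move the pawn.
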(event EventTick
  (params (DeltaSeconds :type Float%20%28single-precision%29))
  (|CallParentFunction DeltaSeconds)
  (Utilities|IsValid (Variables|Default|GetBP_EnemyEye)
    (:Is%20Valid
      (Utilities|IsValid (Variables|Default|GetTargetPawn)
        (:Is%20Valid
          (Development|PrintString (Utilities|String|ToString(Vector) (Math|Vector|GetForwardVector (Math|Rotator|FindLookatRotation (Transformation|GetActorLocation (Variables|Default|GetBP_EnemyEye)) (Transformation|GetActorLocation (Variables|Default|GetTargetPawn)))))))))))

(event EventPossess
  (params (PossessedPawn :type Pawn%20Object%20Reference))
  (bind _asbp_enemy_eye (Utilities|Casting|CastToBP_Enemy_Eye PossessedPawn))
  (Variables|Default|SetBP_EnemyEye _asbp_enemy_eye)
  (Utilities|FlowControl|Delay 0.2)
  (bind _output_get (Variables|Default|SetTargetPawn (Game|Player|GetPlayerPawn 0)))
  (Development|PrintString (Utilities|GetDisplayName _output_get)))

(fn ConstructionScript
  (|CallParentFunction))