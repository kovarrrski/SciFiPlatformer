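; BPC_Vitality is a component that tracks health and defeated state for the actor that owns it.
; BeginPlay fills CurrentHealth from MaxHealth.
; ReceiveDamage subtracts the incoming damage, clamps the result between zero and MaxHealth, and sets IsDefeated when health reaches zero.
; It only stores this state, with no death handling, event dispatch or active Tick logic.
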(event EventBeginPlay
  ;[1 1 1] Set health in the Start
  (Variables|Default|SetCurrentHealth (Variables|Default|GetMaxHealth)))

(event EventTick
  (params (DeltaSeconds :type Float%20%28single-precision%29)))

(fn ReceiveDamage
  (params (Damage :type Float%20%28double-precision%29))
  ;[1 1 1] - Damage (1)
  (Variables|Default|SetCurrentHealth (Math|Float|Clamp(Float) (- (Variables|Default|GetCurrentHealth) Damage) 0.0 (Variables|Default|GetMaxHealth)))
  ;[1 1 1] Check and Set Defeated State
  (if (<= (Variables|Default|GetCurrentHealth) 0.0)
    (Variables|Default|SetIsDefeated true)))